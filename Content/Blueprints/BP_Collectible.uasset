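; BP_Collectible is a pickup that awards one point when the skating player character touches it.
; On BeginPlay a timeline scales its sphere slightly up from normal size as a bounce animation.
; A box overlap by a SkateCharacter adds the point through BP_GameMode, then hides the actor, disables its collision and plays a bubble pop sound.
; The actor is hidden rather than destroyed.
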(event `self.ReceiveBeginPlay`
  (`self.PlayBounceAnim`))

(event `PlayBounceAnim`
  (bind (_direction _alpha) (`Timeline|TL_Bounce` :!via `PlayFromStart`)
    (:`Update`
      (`SceneComponent.SetRelativeScale3D` (`self.Sphere`) (`KismetMathLibrary.VLerp` (1.0 1.0 1.0) (1.2 1.2 1.2) _alpha)))))

(event `self.Box.OnComponentBeginOverlap`
  (params (OverlappedComponent :type "PrimitiveComponent Object Reference") (OtherActor :type "Actor Object Reference") (OtherComp :type "PrimitiveComponent Object Reference") (OtherBodyIndex :type Integer) (bFromSweep :type Boolean) (SweepResult :type "HitResult Structure (by ref)"))
  (cast `SkateCharacter` OtherActor)
  (bind _asbp_game_mode (cast `/Game/Blueprints/BP_GameMode` (`GameplayStatics.GetGameMode`)))
  (`/Game/Blueprints/BP_GameMode.AddPoints` _asbp_game_mode 1)
  (`self.SetActorHiddenInGame` true)
  (`self.SetActorEnableCollision` false)
  (`GameplayStatics.PlaySoundAtLocation` "/Game/Sounds/SFX_Bubble_Pop.SFX_Bubble_Pop" (`self.K2_GetActorLocation`) (struct) 1.0 1.0 0.0 null null null null))

(fn `UserConstructionScript`)