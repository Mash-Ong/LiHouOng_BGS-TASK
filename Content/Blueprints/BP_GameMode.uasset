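; BP_GameMode is the game mode that tracks collectible points and signals when the game is won.
; On BeginPlay it sets the point target to the number of BP_Collectible actors in the level.
; AddPoints raises the running total, calls PointChanged when the value changes, and calls GameWon once the total reaches or exceeds the target.
; GetTotalPoints and GetCurrentPoints expose the target and current count.
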(event `self.ReceiveBeginPlay`
  (bind _outactors (`GameplayStatics.GetAllActorsOfClass` "/Game/Blueprints/BP_Collectible.BP_Collectible_C"))
  (set `self.PointsToCollect` (`KismetArrayLibrary.Array_Length` _outactors)))

(fn `AddPoints`
  (params (PointsToAdd :type Integer))
  (locals (Local_PointBeforeChange :type Integer :default 0))
  (set `local.Local_PointBeforeChange` (`self.CollectedPoints`))
  (set `self.CollectedPoints` (+ (`self.CollectedPoints`) PointsToAdd))
  (`|ExecutionSequence`
    (:`then_0`
      (if (!= (`local.Local_PointBeforeChange`) (`self.CollectedPoints`))
        (`self.PointChanged` (`self.CollectedPoints`))))
    (:`then_1`
      (if (>= (`self.CollectedPoints`) (`self.PointsToCollect`))
        (`self.GameWon`)))))

(fn `GetCurrentPoints`
  (returns (PointsToCollect :type Integer))
  (return (`self.CollectedPoints`)))

(fn `GetTotalPoints`
  (returns (PointsToCollect :type Integer))
  (return (`self.PointsToCollect`)))

(fn `UserConstructionScript`)