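; Skateboarding character Blueprint for Remy that adds a procedural brake pose through play and reverse brake animation events.
; On play, it caches the current mesh location and board rotation, then a timeline lerps the mesh to a fixed X offset and tilts the board's pitch.
; The tilt sign depends on whether the board faces along the control rotation, and reversing plays the same timeline back.
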(event `self.PlayBrakeAnim`
  (bind _output_get (set `self.CacheMeshLoc` (`SceneComponent.RelativeLocation` (`self.Mesh`))))
  (set `self.TargetMeshLoc` (`KismetMathLibrary.MakeVector` -20.0 (.y _output_get) (.z _output_get)))
  (bind _output_get_2 (set `self.CacheBoardLoc` (`SceneComponent.RelativeRotation` (`self.SkateboardRoot`))))
  (set `self.TargetBoardLoc` (`KismetMathLibrary.MakeRotator` (.roll _output_get_2) (`KismetMathLibrary.SelectFloat` 8.0 -8.0 (> (`KismetMathLibrary.Dot_VectorVector` (`SceneComponent.GetForwardVector` (`self.SkateboardRoot`)) (`KismetMathLibrary.GetForwardVector` (`self.GetControlRotation`))) 0.0)) (.yaw _output_get_2)))
  (bind (_direction _loclerpalpha _rotlerpalpha) (`Timeline|TL_BrakeAnim` :!label _label)
    (:`Update`
      (`SceneComponent.K2_SetRelativeLocation` (`self.Mesh`) (`KismetMathLibrary.VLerp` (`self.CacheMeshLoc`) (`self.TargetMeshLoc`) _loclerpalpha) false false)
      (`SceneComponent.K2_SetRelativeRotation` (`self.SkateboardRoot`) (`KismetMathLibrary.RLerp` (`self.CacheBoardLoc`) (`self.TargetBoardLoc`) _rotlerpalpha true) false false))))

(event `self.ReverseBrakeAnim`
  (goto _label :!via `Reverse`))

(fn `UserConstructionScript`)